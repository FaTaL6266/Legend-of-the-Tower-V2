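; Player camera for a tower-building game that pans on WASD, keeps the cursor visible and handles tower placement input.
; Tick polls keys and moves the actor by PanningSpeed, clamping X and Y to XFloat and YFloat.
; Left and right clicks place or destroy the builder tower and re-show the purchase button; ExitGame quits.
; BeginPlay is empty, leaving the BP_Clamp lookup for those bounds disconnected.
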(event `self.ReceiveTick`
  (params (DeltaSeconds :type "Float (single-precision)"))
  (bind _returnvalue (`GameplayStatics.GetPlayerController` 0))
  (bind _panningspeed (`self.PanningSpeed`))
  ;[1 1 1] Camera movement based on user input using WASD.
  ;;[1 1 1] Makes the cursor visible during play.
  (set `PlayerController.bShowMouseCursor` true (`GameplayStatics.GetPlayerController` 0))
  ;;[1 1 1] Sets the movement values based on user input.
  ;;;[1 1 1] Determines if the camera should move left or right based on user input.
  (if (`PlayerController.IsInputKeyDown` _returnvalue "D")
    (set `self.HorizontalPan` 1)
    (elif (`PlayerController.IsInputKeyDown` _returnvalue "A")
      (set `self.HorizontalPan` -1)
      (else
        (set `self.HorizontalPan` 0))))
  ;;;[1 1 1] Determines if the camera should move up or down based on user input.
  (if (`PlayerController.IsInputKeyDown` _returnvalue "W")
    (set `self.VerticalPan` 1)
    (elif (`PlayerController.IsInputKeyDown` _returnvalue "S")
      (set `self.VerticalPan` -1)
      (else
        (set `self.VerticalPan` 0))))
  ;;[1 1 1] Takes the panning value and if the value of either value is not zero, change the location of the camera.
  (if (or (!= (`self.HorizontalPan`) 0) (!= (`self.VerticalPan`) 0))
    ;;[1 1 1] Set the new location of the camera based on user input within the allowed play area.
    (`self.K2_SetActorLocation` (`KismetMathLibrary.MakeVector` (`KismetMathLibrary.FClamp` (.x (+ (`self.K2_GetActorLocation`) (`KismetMathLibrary.MakeVector` (* (`self.VerticalPan`) _panningspeed) (* (`self.HorizontalPan`) _panningspeed)))) (`self.-XFloat`) (`self.+XFloat`)) (`KismetMathLibrary.FClamp` (.y (+ (`self.K2_GetActorLocation`) (`KismetMathLibrary.MakeVector` (* (`self.VerticalPan`) _panningspeed) (* (`self.HorizontalPan`) _panningspeed)))) (`self.-YFloat`) (`self.+YFloat`)) (.z (+ (`self.K2_GetActorLocation`) (`KismetMathLibrary.MakeVector` (* (`self.VerticalPan`) _panningspeed) (* (`self.HorizontalPan`) _panningspeed))))))))

(event `self.ReceiveBeginPlay`
  ;[1 1 1] Sets the valid play area for the game based on inworld location set by the clamp values
)

(event `InputAction|LeftClick`
  (params (Key :type "Key Structure"))
  (bind _buildertowerreference (`self.BuilderTowerReference`))
  ;[1 1 1] On a left click of the mouse, if the BuilderTowerReference is valid, the event PlaceTower in BuilderTowerBP is called.
  (:`Pressed`
    (`/Engine/EditorBlueprintResources/StandardMacros.IsValid` _buildertowerreference
      (:`Is Valid`
        (`/Game/Tower/BP_BuilderTower.Event_PlaceTower` _buildertowerreference)
        (`Widget.SetVisibility` (`/Game/UI/W_Overlay.B_PurchaseTower` (`self.Ref_Widget`)) "Visible")))))

(event `InputAction|RightClick`
  (params (Key :type "Key Structure"))
  (bind _buildertowerreference (`self.BuilderTowerReference`))
  ;[1 1 1] On a right click of the mouse, if the BuilderTowerReference is valid, the event DestroyBuilderTower in BuilderTowerBP is called.
  (:`Pressed`
    (`/Engine/EditorBlueprintResources/StandardMacros.IsValid` _buildertowerreference
      (:`Is Valid`
        (`/Game/Tower/BP_BuilderTower.Event_DestroyBuilderTower` _buildertowerreference)
        (`Widget.SetVisibility` (`/Game/UI/W_Overlay.B_PurchaseTower` (`self.Ref_Widget`)) "Visible")))))

(event `InputAction|ExitGame`
  (params (Key :type "Key Structure"))
  (:`Pressed`
    (`KismetSystemLibrary.QuitGame` null "Quit" true)))

(fn `UserConstructionScript`)