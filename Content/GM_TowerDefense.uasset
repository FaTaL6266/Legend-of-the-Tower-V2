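; Tower defense game mode that tracks the player's lives, money and enemy kill count.
; Custom events subtract lives, add money and deduct money.
; Each money increase also increments the kill count.
; When a life loss brings lives to zero or below, it creates the W_GameOver widget and adds it to the viewport.
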(event `LowerLives`
  (params (ReduceLivesBy :type Integer))
  (bind _lives (`self.Lives`))
  (set `self.Lives` (- _lives ReduceLivesBy))
  (if (<= _lives 0)
    (bind _returnvalue (`|CreateWidget` "/Game/UI/W_GameOVer.W_GameOver_C"))
    (`UserWidget.AddToViewport` _returnvalue 0)))

(event `IncreaseMoney`
  (params (add :type Integer))
  (set `self.Money` (+ add (`self.Money`)))
  (`/Engine/EditorBlueprintResources/StandardMacros.IncrementInt` (`self.EnemiesKilled`)))

(event `DecreaseMoney`
  (params (sub :type Integer))
  (set `self.Money` (- (`self.Money`) sub)))

(fn `UserConstructionScript`)