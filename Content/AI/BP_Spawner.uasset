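; Tower defense wave spawner that spawns enemies at its location and handles those reaching its finish line.
; Chained, self-repeating events spawn Beasts, Zombies, then Mutants on delays, using wave and enemy data tables for counts and stats.
; Tick detects a cleared wave, then shows the spawn-wave button if lives remain, or game over after the final wave.
; Enemies overlapping the FinishLine, placed at EndLocation, deduct lives and are destroyed.
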(event `Event_Mutant`
  (bind _returnvalue (`|GetDataTableRow` "/Game/AI/Data_Wave.Data_Wave" (`KismetStringLibrary.Conv_StringToName` (`KismetStringLibrary.Conv_IntToString` (`self.Wave`))))
    (:`then`
      (bind _returnvalue_2 (`|GetDataTableRow` "/Game/AI/Data_Enemy.Data_Enemy" (`KismetStringLibrary.Conv_StringToName` (`KismetStringLibrary.Conv_IntToString` (`self.TableRow`))))
        (:`then`
          (bind (_beast _beasthealth _beastspeed _zombie _zombiehealth _zombiespeed _mutant _mutanthealth _mutantspeed) (break `/Game/AI/Struct_Wave` _returnvalue))
          (if (== 0 _mutant)
            (set `self.InWave` true)
            (set `self.SpawnCount` 0)
            (set `self.TableRow` 1)
            (else
              (bind (_health _runspeed _spawnspeed _lifededuction _class _mesh) (break `/Game/AI/Struct_Enemy` _returnvalue_2))
              (bind _returnvalue_3 (`AIBlueprintHelperLibrary.SpawnAIFromClass` _class null (`self.K2_GetActorLocation`)))
              (bind _asbp_enemy (cast `/Game/AI/BP_Enemy` _returnvalue_3))
              (`KismetArrayLibrary.Array_Add` (`self.Enemies`) _asbp_enemy)
              (set `/Game/AI/BP_Enemy.Spawner` self _asbp_enemy)
              (set `/Game/AI/BP_Enemy.CurrentHealth` _mutanthealth _asbp_enemy)
              (set `/Game/AI/BP_Enemy.MaxHealth` _mutanthealth _asbp_enemy)
              (set `CharacterMovementComponent.MaxWalkSpeed` _mutantspeed (`Character.CharacterMovement` _asbp_enemy))
              (set `/Game/AI/BP_Enemy.LifeReduction` _lifededuction _asbp_enemy)
              (`SkinnedMeshComponent.SetSkinnedAssetAndUpdate` (`Character.Mesh` _asbp_enemy) _mesh true)
              (`/Engine/EditorBlueprintResources/StandardMacros.IncrementInt` (`self.SpawnCount`)
                (:`  `
                  (`KismetSystemLibrary.Delay` _spawnspeed)
                  (if (== (`self.SpawnCount`) (+ _mutant 1))
                    (set `self.InWave` true)
                    (set `self.SpawnCount` 0)
                    (set `self.TableRow` 1)
                    (elif (== 0 _mutant)
                      (set `self.InWave` true)
                      (set `self.SpawnCount` 0)
                      (set `self.TableRow` 1)
                      (else
                        (`self.Event_Mutant`)))))))))))))

(event `Event_Zombie`
  (bind _returnvalue (`|GetDataTableRow` "/Game/AI/Data_Wave.Data_Wave" (`KismetStringLibrary.Conv_StringToName` (`KismetStringLibrary.Conv_IntToString` (`self.Wave`))))
    (:`then`
      (bind _returnvalue_2 (`|GetDataTableRow` "/Game/AI/Data_Enemy.Data_Enemy" (`KismetStringLibrary.Conv_StringToName` (`KismetStringLibrary.Conv_IntToString` (`self.TableRow`))))
        (:`then`
          (bind (_beast _beasthealth _beastspeed _zombie _zombiehealth _zombiespeed) (break `/Game/AI/Struct_Wave` _returnvalue))
          (if (== 0 _zombie)
            (set `self.SpawnCount` 0)
            (`self.Event_Mutant`)
            (`/Engine/EditorBlueprintResources/StandardMacros.IncrementInt` (`self.TableRow`))
            (else
              (bind (_health _runspeed _spawnspeed _lifededuction _class _mesh) (break `/Game/AI/Struct_Enemy` _returnvalue_2))
              (bind _returnvalue_3 (`AIBlueprintHelperLibrary.SpawnAIFromClass` _class null (`self.K2_GetActorLocation`)))
              (bind _asbp_enemy (cast `/Game/AI/BP_Enemy` _returnvalue_3))
              (`KismetArrayLibrary.Array_Add` (`self.Enemies`) _asbp_enemy)
              (set `/Game/AI/BP_Enemy.Spawner` self _asbp_enemy)
              (set `/Game/AI/BP_Enemy.CurrentHealth` _zombiehealth _asbp_enemy)
              (set `/Game/AI/BP_Enemy.MaxHealth` _zombiehealth _asbp_enemy)
              (set `CharacterMovementComponent.MaxWalkSpeed` _zombiespeed (`Character.CharacterMovement` _asbp_enemy))
              (set `/Game/AI/BP_Enemy.LifeReduction` _lifededuction _asbp_enemy)
              (`SkinnedMeshComponent.SetSkinnedAssetAndUpdate` (`Character.Mesh` _asbp_enemy) _mesh true)
              (`/Engine/EditorBlueprintResources/StandardMacros.IncrementInt` (`self.SpawnCount`)
                (:`  `
                  (`KismetSystemLibrary.Delay` _spawnspeed)
                  (if (== (`self.SpawnCount`) _zombie)
                    (set `self.SpawnCount` 0)
                    (`self.Event_Mutant`)
                    (`/Engine/EditorBlueprintResources/StandardMacros.IncrementInt` (`self.TableRow`))
                    (else
                      (`self.Event_Zombie`))))))))))))

(event `Event_Beast`
  (bind _returnvalue (`|GetDataTableRow` "/Game/AI/Data_Wave.Data_Wave" (`KismetStringLibrary.Conv_StringToName` (`KismetStringLibrary.Conv_IntToString` (`self.Wave`))))
    (:`then`
      (bind _returnvalue_2 (`|GetDataTableRow` "/Game/AI/Data_Enemy.Data_Enemy" (`KismetStringLibrary.Conv_StringToName` (`KismetStringLibrary.Conv_IntToString` (`self.TableRow`))))
        (:`then`
          (bind (_beast _beasthealth _beastspeed) (break `/Game/AI/Struct_Wave` _returnvalue))
          (if (== 0 _beast)
            (set `self.SpawnCount` 0)
            (`self.Event_Zombie`)
            (`/Engine/EditorBlueprintResources/StandardMacros.IncrementInt` (`self.TableRow`))
            (else
              (bind (_health _runspeed _spawnspeed _lifededuction _class _mesh) (break `/Game/AI/Struct_Enemy` _returnvalue_2))
              (bind _returnvalue_3 (`AIBlueprintHelperLibrary.SpawnAIFromClass` _class null (`self.K2_GetActorLocation`)))
              (bind _asbp_enemy (cast `/Game/AI/BP_Enemy` _returnvalue_3))
              (`KismetArrayLibrary.Array_Add` (`self.Enemies`) _asbp_enemy)
              (set `/Game/AI/BP_Enemy.Spawner` self _asbp_enemy)
              (set `/Game/AI/BP_Enemy.CurrentHealth` _beasthealth _asbp_enemy)
              (set `/Game/AI/BP_Enemy.MaxHealth` _beasthealth _asbp_enemy)
              (set `CharacterMovementComponent.MaxWalkSpeed` _beastspeed (`Character.CharacterMovement` _asbp_enemy))
              (set `/Game/AI/BP_Enemy.LifeReduction` _lifededuction _asbp_enemy)
              (`SkinnedMeshComponent.SetSkinnedAssetAndUpdate` (`Character.Mesh` _asbp_enemy) _mesh true)
              (`/Engine/EditorBlueprintResources/StandardMacros.IncrementInt` (`self.SpawnCount`)
                (:`  `
                  (`KismetSystemLibrary.Delay` _spawnspeed)
                  (if (== (`self.SpawnCount`) (- _beast 1))
                    (set `self.SpawnCount` 0)
                    (`self.Event_Zombie`)
                    (`/Engine/EditorBlueprintResources/StandardMacros.IncrementInt` (`self.TableRow`))
                    (else
                      (`self.Event_Beast`))))))))))))

(event `Event_CreateSpawnWaveButton`
  (if (> (`self.Wave`) 20)
    (bind _returnvalue (`|CreateWidget` "/Game/UI/W_GameOver.W_GameOver_C"))
    (`UserWidget.AddToViewport` _returnvalue 0)
    (elif (> (`/Game/GM_TowerDefense.Lives` (`self.Ref_GameMode`)) 0)
      (`Widget.SetVisibility` (`/Game/UI/W_Overlay.B_SpawnWave` (`self.Ref_Widget`)) "Visible")
      (set `/Game/UI/W_Overlay.Ref_Spawner` self (`self.Ref_Widget`)))))

(event `self.ReceiveTick`
  (params (DeltaSeconds :type "Float (single-precision)"))
  (if (and (== (`KismetArrayLibrary.Array_Length` (`self.Enemies`)) 0) (`self.InWave`))
    (set `self.InWave` false)
    (`/Engine/EditorBlueprintResources/StandardMacros.IncrementInt` (`self.Wave`)
      (:`  `
        (`self.Event_CreateSpawnWaveButton`)))))

(event `self.ReceiveBeginPlay`
  (bind _asgm_tower_defense (cast `/Game/GM_TowerDefense` (`GameplayStatics.GetGameMode`)))
  (set `self.Ref_GameMode` _asgm_tower_defense))

(event `self.FinishLine.OnComponentBeginOverlap`
  (params (OverlappedComponent :type "PrimitiveComponent Object Reference") (OtherActor :type "Actor Object Reference") (OtherComp :type "PrimitiveComponent Object Reference") (OtherBodyIndex :type Integer) (bFromSweep :type Boolean) (SweepResult :type "HitResult Structure (by ref)"))
  (bind _asbp_enemy (cast `/Game/AI/BP_Enemy` OtherActor))
  (bind _asgm_tower_defense (cast `/Game/GM_TowerDefense` (`GameplayStatics.GetGameMode`)))
  (`/Game/GM_TowerDefense.LowerLives` _asgm_tower_defense (`/Game/AI/BP_Enemy.LifeReduction` _asbp_enemy))
  (`KismetArrayLibrary.Array_RemoveItem` (`self.Enemies`) _asbp_enemy)
  (`self.K2_DestroyActor` _asbp_enemy))

(fn `UserConstructionScript`
  (`SceneComponent.K2_SetRelativeLocation` (`self.FinishLine`) (`self.EndLocation`) false false))