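; BP_Enemy is a tower defense enemy (AI runner) that takes damage and pays out money when killed.
; On BeginPlay it passes itself to its W_Healthbar widget as the runner reference.
; AnyDamage lowers CurrentHealth, and at zero or below removes the enemy from its Spawner's AliveRunners list and destroys it.
; It then adds its Money value to the player's funds through GM_TowerDefense.
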(event `self.ReceiveBeginPlay`
  (bind _asw_healthbar (cast `/Game/UI/W_HealthBar` (`WidgetComponent.GetUserWidgetObject` (`self.EnemyHealthBar`))))
  (set `/Game/UI/W_HealthBar.AIRunnerReference` self _asw_healthbar))

(event `self.ReceiveAnyDamage`
  (params (Damage :type "Float (single-precision)") (DamageType :type "DamageType Object Reference") (InstigatedBy :type "Controller Object Reference") (DamageCauser :type "Actor Object Reference"))
  ;[1 1 1] When the AIRunner receives damage, the damage is subtracted from the health of the AIRunner. If the health of th AIRunner is equal to or less than 0, the AIRunner is destroyed.
  (bind _output_get (set `self.CurrentHealth` (- (`self.CurrentHealth`) Damage)))
  (if (<= _output_get 0.0)
    (`KismetArrayLibrary.Array_RemoveItem` (`/Game/AI/BP_Spawner.AliveRunners` (`self.Spawner`)) self)
    (`self.K2_DestroyActor`)
    ;[1 1 1] Add cash on kill
    (bind _asgm_tower_defense (cast `/Game/GM_TowerDefense` (`GameplayStatics.GetGameMode`)))
    (`/Game/GM_TowerDefense.IncreaseMoney` _asgm_tower_defense (`self.Money`))))

(fn `UserConstructionScript`)